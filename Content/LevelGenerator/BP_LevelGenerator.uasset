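; BP_LevelGenerator builds a grid-based maze level on BeginPlay by spawning tile actors at scaled cell positions.
; GenMaze first destroys previously tracked actors through ClearMaze, then loops over the grid and records each new spawn in GenActors.
; Each cell uses the Default class, or by SpecialRate chance a random class from Library, except the four corners, which always stay Default.
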(event EventBeginPlay
  (CallFunction|GenMaze))

(event Collision|EventActorBeginOverlap
  (params (OtherActor :type Actor%20Object%20Reference)))

(event EventTick
  (params (DeltaSeconds :type Float%20%28single-precision%29)))

(fn ConstructionScript)

(fn ClearMaze
  (for _array_element (Variables|Default|GetgenActors)
    (Actor|DestroyActor _array_element))
  (Variables|Default|SetgenActors (Utilities|Array|MakeArray))
  (Development|PrintString "Empty Ref Array"))

(fn GenMaze
  (bind _size (Variables|Default|Getsize))
  (bind _size_2 (Variables|Default|Getsize))
  (bind _returnvalue (Math|Conversions|ToFloat(Integer) _size_2))
  (CallFunction|ClearMaze)
  (for _index (range 0 _size)
    (for _index_2 (range 0 _size)
      (if (<= (Math|Random|RandomFloat) (Variables|Default|GetspecialRate))
        (if (> (Utilities|Array|Length (Variables|Default|Getlibrary)) 0)
          (if (Utilities|Array|ContainsItem (Utilities|Array|MakeArray (Math|Vector2D|MakeVector2D 0.0 0.0) (Math|Vector2D|MakeVector2D 0.0 _returnvalue) (Math|Vector2D|MakeVector2D _returnvalue _returnvalue) (Math|Vector2D|MakeVector2D _returnvalue 0.0)) (Math|Conversions|ToVector2D(Vector) (Math|Vector|MakeVector (Math|Conversions|ToFloat(Integer) _index_2) (Math|Conversions|ToFloat(Integer) _index) 0.0)))
            (Development|PrintString (Utilities|String|ToString(Vector2d) (Math|Conversions|ToVector2D(Vector) (Math|Vector|MakeVector (Math|Conversions|ToFloat(Integer) _index_2) (Math|Conversions|ToFloat(Integer) _index) 0.0))))
            (bind _returnvalue_2 (Game|SpawnActorfromClass (Variables|Default|Getdefault) (Math|Transform|MakeTransform (* (Math|Vector|MakeVector (Math|Conversions|ToFloat(Integer) _index_2) (Math|Conversions|ToFloat(Integer) _index) 0.0) (Variables|Default|Getscale))) "Undefined" "MultiplyWithRoot" self 0 :!label _label))
            (Utilities|IsValid _returnvalue_2
              (:Is%20Valid
                (Utilities|Array|Add (Variables|Default|GetgenActors) _returnvalue_2))
              (:Is%20Not%20Valid
                (Development|PrintString "Fail to spawn actor")))
            (else
              (bind _returnvalue_3 (Game|SpawnActorfromClass (.OutItem (Utilities|Array|Random (Variables|Default|Getlibrary))) (Math|Transform|MakeTransform (* (Math|Vector|MakeVector (Math|Conversions|ToFloat(Integer) _index_2) (Math|Conversions|ToFloat(Integer) _index) 0.0) (Variables|Default|Getscale))) "Undefined" "MultiplyWithRoot" self 0))
              (Utilities|IsValid _returnvalue_3
                (:Is%20Valid
                  (Utilities|Array|Add (Variables|Default|GetgenActors) _returnvalue_3))
                (:Is%20Not%20Valid
                  (Development|PrintString "Fail to spawn actor")))))
          (else
            (goto _label)))
        (else
          (goto _label))))))