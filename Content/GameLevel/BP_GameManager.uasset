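; Game manager actor that detects the end of a round in GameLevel and announces the result.
; Every Tick, CheckAlive counts BP_Player actors whose mesh is not simulating physics, treating ragdolled players as dead.
; With one or none left, it shows UW_RoundEndOverlay naming the winner or a draw, then reopens GameLevel after a short Delay.
; Tick has no game-over guard, so overlays are added every frame until the reload.
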(event EventBeginPlay)

(event Collision|EventActorBeginOverlap
  (params (OtherActor :type Actor%20Object%20Reference)))

(event EventTick
  (params (DeltaSeconds :type Float%20%28single-precision%29))
  (bind (_isgameover _lastplayer) (CallFunction|CheckAlive))
  (if _isgameover
    (Utilities|IsValid _lastplayer
      (:Is%20Valid
        (bind _returnvalue (UserInterface|CreateWidget "/Game/UI/RoundEndOverlay/UW_RoundEndOverlay.UW_RoundEndOverlay_C"))
        (Variables|/Script/UMG.TextBlock|SetText (Variables|/Game/UI/RoundEndOverlay/UW_RoundEndOverlay.UW_RoundEndOverlay_C|GetRoundMsg _returnvalue) (Utilities|Text|ToText(String) (Utilities|String|Append "Round Over. 
" (Utilities|GetDisplayName _lastplayer) " Wins!")))
        (UserInterface|Viewport|AddtoViewport _returnvalue 0))
      (:Is%20Not%20Valid
        (bind _returnvalue_2 (UserInterface|CreateWidget "/Game/UI/RoundEndOverlay/UW_RoundEndOverlay.UW_RoundEndOverlay_C"))
        (Variables|/Script/UMG.TextBlock|SetText (Variables|/Game/UI/RoundEndOverlay/UW_RoundEndOverlay.UW_RoundEndOverlay_C|GetRoundMsg _returnvalue_2) "Round Over. 
Draw. You all suck!")
        (UserInterface|Viewport|AddtoViewport _returnvalue_2 0)))
    (Utilities|FlowControl|Delay 3.0)
    (Game|OpenLevel(byName) "GameLevel")))

(fn ConstructionScript)

(fn CheckAlive
  (bind _outactors (Actor|GetAllActorsOfClass "/Game/Gameplay/Player/Blueprints/BP_Player.BP_Player_C"))
  (for _array_element _outactors
    (if (not (Class|SceneComponent|IsAnySimulatingPhysics (Variables|/Script/Engine.Character|GetMesh _array_element)))
      (Math|Integer|IncrementInt (LocalVariables|GetplayersAlive)
        (:%20%20
          (LocalVariables|SetlastPlayerAlive _array_element)))))
  (return (<= (LocalVariables|GetplayersAlive) 1) (LocalVariables|GetlastPlayerAlive)))