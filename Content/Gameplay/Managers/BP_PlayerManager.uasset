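; BP_PlayerManager creates local players at level start from the player data stored in the GI_Stacked game instance.
; On BeginPlay it loops over the keys of the Players map and calls CreatePlayer with each entry's stored controller ID, spawning a player controller.
; Debug prints log pawn, controller and local player state, each creation, missing entries and an unexpected game instance type.
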(event EventBeginPlay
  (bind _asgi_stacked (Utilities|Casting|CastToGI_Stacked (Game|GetGameInstance))
    (:then
      (bind _keys (Utilities|Map|Keys (Variables|/Game/Gameplay/GI_Stacked.GI_Stacked_C|Getplayers _asgi_stacked)))
      (for _array_element _keys
        (Development|PrintString (Utilities|String|Append (Utilities|String|ToString(Integer) 0) " Player ID; " (Utilities|GetDisplayName (Game|Player|GetPlayerPawn _array_element)) "; Controller ID = " (Utilities|String|ToString(Integer) (Class|GameplayStatics|GetPlayerControllerID (Game|GetPlayerController _array_element))) "; Num Local = " (Utilities|String|ToString(Integer) (Class|GameplayStatics|GetNumLocalPlayerControllers)) "; Posessed = " (Utilities|GetDisplayName (Pawn|GetControlledPawn (Game|GetPlayerController _array_element)))))
        (if (.ReturnValue (Utilities|Map|Find (Variables|/Game/Gameplay/GI_Stacked.GI_Stacked_C|Getplayers _asgi_stacked) _array_element))
          (bind _returnvalue (Class|GameplayStatics|CreatePlayer (.playercontrollerid (.Value (Utilities|Map|Find (Variables|/Game/Gameplay/GI_Stacked.GI_Stacked_C|Getplayers _asgi_stacked) _array_element)))))
          (Development|PrintString (Utilities|String|Append "create " (.nickname (.Value (Utilities|Map|Find (Variables|/Game/Gameplay/GI_Stacked.GI_Stacked_C|Getplayers _asgi_stacked) _array_element))) " - " (Utilities|GetDisplayName _returnvalue) "@ Player (" (Utilities|String|ToString(Integer) _array_element) ") & Controller (" (Utilities|String|ToString(Integer) (.playercontrollerid (.Value (Utilities|Map|Find (Variables|/Game/Gameplay/GI_Stacked.GI_Stacked_C|Getplayers _asgi_stacked) _array_element)))) ")"))
          (else
            (Development|PrintString (Utilities|String|BuildString(Integer) "NO Player defined @ Player Index =" "" _array_element))))
        (Development|PrintString "-----------------")))
    (:CastFailed
      (Development|PrintString "UNEXPECTED GI"))))

(event Collision|EventActorBeginOverlap
  (params (OtherActor :type Actor%20Object%20Reference)))

(event EventTick
  (params (DeltaSeconds :type Float%20%28single-precision%29)))

(fn ConstructionScript)