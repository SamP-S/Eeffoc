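; BP_DebugManager is a debug manager that prints local multiplayer player and controller information to the screen.
; On BeginPlay it starts a looping timer that fires PrintPlayers every few seconds.
; PrintPlayers loops over four player indices, printing each pawn's display name, its controller ID and the local player controller count, followed by a separator line.
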(event Custom|PrintPlayers
  (for _index (range 0 3)
    (Development|PrintString (Utilities|String|Append (Utilities|String|ToString(Integer) _index) " Player ID; " (Utilities|GetDisplayName (Game|Player|GetPlayerPawn _index)) "; Controller ID =" (Utilities|String|ToString(Integer) (Class|GameplayStatics|GetPlayerControllerID (Game|GetPlayerController _index))) "; Num Local = " (Utilities|String|ToString(Integer) (Class|GameplayStatics|GetNumLocalPlayerControllers))))
    (Development|PrintString "-----------------")))

(event EventBeginPlay
  (Utilities|Time|SetTimerbyEvent (delegate Custom|PrintPlayers) 3.0 true))

(fn ConstructionScript)