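; BP_BaseCharacter is a base character Blueprint that loads its stats from the DT_Characters data table.
; BeginPlay passes CharacterName to SetCharacter, which stores it and calls TrySetCharacter to look up a row and fill BaseHealth, BaseSpeed and Material.
; SetCharacter passes an empty string to TrySetCharacter, so the lookup does not use the stored name.
; A missing row only prints a failure message.
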(event Custom|SetCharacter
  (params (CharacterName :type String))
  (Variables|Default|SetcharacterName CharacterName)
  (CallFunction|TrySetCharacter))

(event EventBeginPlay
  (CallFunction|SetCharacter (Variables|Default|GetcharacterName)))

(event Collision|EventActorBeginOverlap
  (params (OtherActor :type Actor%20Object%20Reference)))

(event EventTick
  (params (DeltaSeconds :type Float%20%28single-precision%29)))

(fn ConstructionScript)

(fn TrySetCharacter
  (params (CharacterName :type String))
  (bind _returnvalue (Utilities|GetDataTableRow "/Game/Gameplay/Characters/DT_Characters.DT_Characters" (Utilities|String|StringToName CharacterName))
    (:then
      (Variables|Default|SetbaseHealth (.health (Utilities|Struct|BreakS_CharacterProperties _returnvalue)))
      (Variables|Default|SetbaseSpeed (.speed (Utilities|Struct|BreakS_CharacterProperties _returnvalue)))
      (Variables|Default|Setmaterial (.health100 (Utilities|Struct|BreakS_CharacterProperties _returnvalue))))
    (:RowNotFound
      (Development|PrintString (Utilities|String|Append "FAILED to load character: " "")))))