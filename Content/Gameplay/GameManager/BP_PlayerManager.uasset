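; BP_PlayerManager creates the local players registered in the game instance when play begins.
; It casts the game instance to GI_Stacked and spawns a player with its own controller for each key in the Players map, using the key as the controller ID.
; It then prints the pawns for the first four player indices as debug output, or an error message if the cast fails.
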(event EventBeginPlay
  (bind _asgi_stacked (Utilities|Casting|CastToGI_Stacked (Game|GetGameInstance))
    (:then
      (bind _keys (Utilities|Map|Keys (Variables|/Game/Gameplay/GI_Stacked.GI_Stacked_C|Getplayers _asgi_stacked)))
      (for _array_element _keys
        (bind _returnvalue (Class|GameplayStatics|CreatePlayer _array_element)))
      (for _index (range 0 3)
        (Development|PrintString (Utilities|String|Append (Utilities|GetDisplayName (Game|Player|GetPlayerPawn _index)) " @ " (Utilities|String|ToString(Integer) _index)))))
    (:CastFailed
      (Development|PrintString "UNEXPECTED GI"))))

(event Collision|EventActorBeginOverlap
  (params (OtherActor :type Actor%20Object%20Reference)))

(event EventTick
  (params (DeltaSeconds :type Float%20%28single-precision%29)))

(fn ConstructionScript)