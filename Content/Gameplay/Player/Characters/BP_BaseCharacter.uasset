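; BP_BaseCharacter is the base player character, which configures itself from a named row in DT_Characters.
; When the controller changes, it looks up the local player by player controller ID in GI_BoomeRounds and takes that player's character name.
; TrySetCharacter stores the row's base health and speed and applies its full-health skin material to the mesh.
; SetCharacterByName stores a given name but passes an empty string to that lookup.
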(event Custom|SetCharacterByLocalPlayer
  (params (localPlayer :type S%20Local%20Player%20Structure))
  (bind _output_get (Variables|Default|SetcharacterName (.characterName (Utilities|Struct|BreakS_LocalPlayer localPlayer))))
  (CallFunction|TrySetCharacter _output_get))

(event Custom|SetCharacterByName
  (params (CharacterName :type String))
  (Variables|Default|SetcharacterName CharacterName)
  (CallFunction|TrySetCharacter))

(event EventBeginPlay)

(event Collision|EventActorBeginOverlap
  (params (OtherActor :type Actor%20Object%20Reference)))

(event EventTick
  (params (DeltaSeconds :type Float%20%28single-precision%29)))

(event EventControllerChanged
  (params (OldController :type Controller%20Object%20Reference) (NewController :type Controller%20Object%20Reference))
  (Utilities|IsValid NewController
    (:Is%20Valid
      (bind _asplayer_controller (Utilities|Casting|CastToPlayerController NewController)
        (:then
          (bind _asgi_boome_rounds (Utilities|Casting|CastToGI_BoomeRounds (Game|GetGameInstance))
            (:then
              (if (.ReturnValue (Utilities|Map|Find (Variables|/Game/Gameplay/Global/GI_BoomeRounds.GI_BoomeRounds_C|GetsLocalPlayers _asgi_boome_rounds) (Class|GameplayStatics|GetPlayerControllerID _asplayer_controller)))
                (CallFunction|SetCharacterbyLocalPlayer (.Value (Utilities|Map|Find (Variables|/Game/Gameplay/Global/GI_BoomeRounds.GI_BoomeRounds_C|GetsLocalPlayers _asgi_boome_rounds) (Class|GameplayStatics|GetPlayerControllerID _asplayer_controller))))
                (else
                  (Development|PrintString (Utilities|String|BuildString(Integer) "NO LocalPlayyer Found for PlayerControllerID" " = " (Class|GameplayStatics|GetPlayerControllerID _asplayer_controller))))))
            (:CastFailed
              (Development|PrintString "GI is not BOOMEROUNDS"))))
        (:CastFailed
          (Development|PrintString "Controller is NOT Player Controller"))))))

(fn ConstructionScript)

(fn TrySetCharacter
  (params (CharacterName :type String))
  (bind _returnvalue (Utilities|GetDataTableRow "/Game/Gameplay/Player/Characters/DT_Characters.DT_Characters" (Utilities|String|StringToName CharacterName))
    (:then
      (Variables|Default|SetbaseHealth (.charHealth (Utilities|Struct|BreakS_CharacterProperties _returnvalue)))
      (Variables|Default|SetbaseSpeed (.charSpeed (Utilities|Struct|BreakS_CharacterProperties _returnvalue)))
      (bind _output_get (Variables|Default|Setmaterial (.charSkinFullHealth (Utilities|Struct|BreakS_CharacterProperties _returnvalue))))
      (Rendering|Material|SetMaterial (Variables|Character|GetMesh) 0 _output_get)
      (Development|PrintString (Utilities|String|Append "Set Character: " CharacterName)))
    (:RowNotFound
      (Development|PrintString (Utilities|String|Append "FAILED to load character: " "")))))