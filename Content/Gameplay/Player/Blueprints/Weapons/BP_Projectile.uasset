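; Weapon projectile that damages a player it hits, applies an impulse to their mesh, and destroys itself on any hit.
; When ShouldExpload is set and its owner is a player, BoomBoom spawns explosion effects and runs a sphere trace.
; The blast kills and launches players other than the owner, and enables physics on listed meshes in BP_DestructableSquare actors, pushing them outward.
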(event Collision|EventHit
  (params (MyComp :type Primitive%20Component%20Object%20Reference) (Other :type Actor%20Object%20Reference) (OtherComp :type Primitive%20Component%20Object%20Reference) (bSelfMoved :type Boolean) (HitLocation :type Vector :default "0, 0, 0") (HitNormal :type Vector :default "0, 0, 0") (NormalImpulse :type Vector :default "0, 0, 0") (Hit :type Hit%20Result%20Structure%20%28by%20ref%29))
  (Utilities|FlowControl|Sequence
    (:then_0
      (bind _asbp_player (Utilities|Casting|CastToBP_Player (.hitactor Hit)))
      (Default|Hit _asbp_player 3e+01)
      (Physics|AddImpulseatLocation (Variables|/Script/Engine.Character|GetMesh _asbp_player) (Utilities|GetImpulse) (Transformation|GetActorLocation) "None"))
    (:then_1
      (if (Variables|Default|GetshouldExpload)
        (bind _asbp_player_2 (Utilities|Casting|CastToBP_Player (Components|GetOwner))
          (:then
            (CallFunction|BoomBoom _asbp_player_2 (.location Hit)))
          (:CastFailed
            (Development|PrintString "BP_projectile: uh oh fucky wucky")))))
    (:then_2
      (Actor|DestroyActor) ; Then destroy this projectile
    )))

(fn ConstructionScript)

(fn BoomBoom
  (params (Player :type BP%20Player%20Object%20Reference) (Location :type Vector))
  (Development|PrintString (Utilities|GetDisplayName Player))
  (Effects|SpawnEmitteratLocation "/Game/StarterContent/Particles/P_Explosion.P_Explosion" Location "0, 0, 0" "5.000000,5.000000,5.000000")
  (Audio|PlaySoundatLocation "/Game/StarterContent/Audio/Explosion01.Explosion01" Location "0, 0, 0" 1.0 1.0 0.0 0 0 0 0)
  (Utilities|FlowControl|Sequence
    (:then_0
      (bind _outhits (Collision|MultiSphereTraceByChannel Location Location 2.5e+02 "TraceTypeQuery1" false 0 "None" false))
      (for _array_element _outhits
        (bind _asbp_player (Utilities|Casting|CastToBP_Player (.hitactor _array_element))
          (:then
            (Development|PrintString (Utilities|String|Append "BoomBoom: " (Utilities|GetDisplayName Player) "->" (Utilities|GetDisplayName (.hitactor _array_element))))
            (if (!= Player _asbp_player)
              (Default|KillPlayer _asbp_player)
              (Physics|AddImpulseatLocation (Variables|/Script/Engine.Character|GetMesh _asbp_player) (* (Math|Vector|Normalize (- Location (Transformation|GetActorLocation _asbp_player))) -5e+04) Location "None")))
          (:CastFailed
            (bind _asbp_destructable_square (Utilities|Casting|CastToBP_DestructableSquare (.hitactor _array_element)))
            (for _array_element_2 (Actor|GetComponentsByClass _asbp_destructable_square "/Script/Engine.StaticMeshComponent")
              (if (Utilities|Set|Contains (Variables|Default|GetdestructableActors) (Variables|/Script/Engine.StaticMeshComponent|GetStaticMesh _array_element_2))
                (Physics|SetSimulatePhysics _array_element_2 true)
                (Physics|AddImpulseatLocation _array_element_2 (* (Math|Vector|Normalize (- Location (Transformation|GetActorLocation _asbp_destructable_square))) -5e+04) Location "None")))))))))