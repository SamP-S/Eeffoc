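; BP_Explosion is a short-lived explosion actor that ragdolls and launches nearby BP_Player characters.
; On BeginPlay it plays a scaled particle effect and sound, then runs a sphere trace at its location.
; Each BP_Player hit, except the one stored in Player, gets mesh physics, loses capsule collision and movement, and receives an impulse away from the blast.
; The actor destroys itself after a brief delay.
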(event EventBeginPlay
  (bind _returnvalue (Transformation|GetActorLocation))
  (bind _returnvalue_2 (Transformation|GetActorLocation))
  (Effects|SpawnEmitteratLocation "/Game/StarterContent/Particles/P_Explosion.P_Explosion" (Transformation|GetActorLocation) "0, 0, 0" "5.000000,5.000000,5.000000")
  (Audio|PlaySoundatLocation "/Game/StarterContent/Audio/Explosion01.Explosion01" (Transformation|GetActorLocation) "0, 0, 0" 1.0 1.0 0.0 0 0 0 0)
  (Utilities|FlowControl|Sequence
    (:then_0
      (bind _outhits (Collision|MultiSphereTraceByChannel _returnvalue_2 _returnvalue_2 2.5e+02 "TraceTypeQuery1" false 0 "None" false))
      (for _array_element _outhits
        (bind _asbp_player (Utilities|Casting|CastToBP_Player (.hitactor _array_element)))
        (if (!= (Variables|Default|GetPlayer) _asbp_player)
          (Class|SkeletalMeshComponent|SetAllBodiesSimulatePhysics (Variables|/Script/Engine.Character|GetMesh _asbp_player) true)
          (Collision|SetCollisionEnabled (Variables|/Script/Engine.Character|GetCapsuleComponent _asbp_player) "NoCollision")
          (Pawn|Components|CharacterMovement|DisableMovement (Variables|/Script/Engine.Character|GetCharacterMovement _asbp_player))
          (Physics|AddImpulseatLocation (Variables|/Script/Engine.Character|GetMesh _asbp_player) (* (Math|Vector|Normalize (- _returnvalue (Transformation|GetActorLocation _asbp_player))) -5e+04) _returnvalue "None"))))
    (:then_1
      (Utilities|FlowControl|Delay 0.1)
      (Actor|DestroyActor))))

(fn ConstructionScript)