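; BP_Card is an early-stage player card Blueprint that listens for health changes on a BP_Player.
; On BeginPlay it gathers all BP_Player actors, takes the one at index 1 and binds to its health-change dispatcher.
; The bound event only prints the player's name and current health as debug output.
; Its attach and detach player handlers are empty stubs.
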(event Custom|OnHealthChange
  (bind _player (Variables|Default|Getplayer))
  (Development|PrintString (Utilities|String|Append "OnHealthChange " (Utilities|GetDisplayName _player) ": " (Utilities|String|ToString(Float) (Variables|/Game/Gameplay/Player/BP_Player.BP_Player_C|GetcurHealth _player)))))

(event EventBeginPlay
  (bind _outactors (Actor|GetAllActorsOfClass "/Game/Gameplay/Player/BP_Player.BP_Player_C"))
  (bind _output_get (Variables|Default|Setplayer (Utilities|Array|Get(acopy) _outactors 1)))
  (EventDispatchers|BindEventtoOnHealthChange _output_get (delegate Custom|OnHealthChange))
  (Development|PrintString (Utilities|String|Append (Utilities|GetDisplayName _output_get) " BIND")))

(event Collision|EventActorBeginOverlap
  (params (OtherActor :type Actor%20Object%20Reference)))

(event EventTick
  (params (DeltaSeconds :type Float%20%28single-precision%29)))

(fn ConstructionScript)

(fn OnAttachPlayerHandler
  (params (Player :type BP%20Player%20Object%20Reference)))

(fn OnDetachPlayerHandler)