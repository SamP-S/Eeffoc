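; Shared orthographic camera that follows all living BP_Player actors and becomes player 0's view target on BeginPlay.
; Each tick it eases toward the players' average position, scaled from a center point by a follow strength.
; When zoom is enabled, it projects every player to normalized screen space and widens or narrows OrthoWidth based on the closest distance to a screen edge, using two thresholds as a dead band.
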(event EventBeginPlay
  (Game|Player|SetViewTargetwithBlend (Game|GetPlayerController 0) self 0.0 "VTBlend_Linear" 0.0 false)
  (Development|PrintText "Set CAMERA"))

(event EventTick
  (params (DeltaSeconds :type Float%20%28single-precision%29))
  (bind _avgposition (CallFunction|GetPlayerAvgPosition))
  (Transformation|SetActorLocation (Math|Interpolation|VInterpTo (Transformation|GetActorLocation) (Utilities|GetFollowPosition _avgposition) DeltaSeconds 0.0) false false)
  (CallFunction|TryZoom))

(fn ConstructionScript)

(fn GetPlayerAvgPosition
  (bind _outactors (Actor|GetAllActorsOfClass "/Game/Gameplay/Player/Blueprints/BP_Player.BP_Player_C"))
  (for _array_element _outactors
    (if (Variables|/Game/Gameplay/Player/Blueprints/BP_Player.BP_Player_C|GetisAlive _array_element)
      (LocalVariables|Set%20newPos (+ (LocalVariables|Get%20newPos) (.location (Transformation|GetActorTransform _array_element))))
      (Math|Integer|IncrementInt (LocalVariables|GetplayerCount))))
  (if (!= (LocalVariables|GetplayerCount) 0)
    (return (/ (LocalVariables|Get%20newPos) (LocalVariables|GetplayerCount)))))

(fn Zoom
  (params (isZoomIn :type Boolean))
  (bind _camera (Variables|Default|GetCamera))
  (Class|CameraComponent|SetOrthoWidth _camera (+ (* (Variables|Default|GetzoomSpeed) (Math|Integer|SelectInt -1 1 isZoomIn) (Utilities|Time|GetWorldDeltaSeconds)) (Variables|/Script/Engine.CameraComponent|GetOrthoWidth _camera))))

(fn GetPlayersMinDist
  (bind _outactors (Actor|GetAllActorsOfClass "/Game/Gameplay/Player/Blueprints/BP_Player.BP_Player_C"))
  (for _array_element _outactors
    (if (< (Utilities|ScreenFtoMinDist (Utilities|WorldtoScreenF (Transformation|GetActorLocation _array_element))) (LocalVariables|GetminDist))
      (LocalVariables|SetminDist (Utilities|ScreenFtoMinDist (Utilities|WorldtoScreenF (Transformation|GetActorLocation _array_element))))))
  (return (LocalVariables|GetminDist)))

(fn TryZoom
  (if (Variables|Default|GetisZoomEnabled)
    (bind _playersmindist (CallFunction|GetPlayersMinDist))
    (if (< _playersmindist (Variables|Default|GetzoomOutLimit))
      (CallFunction|Zoom false)
      (elif (> _playersmindist (Variables|Default|GetzoomInLimit))
        (CallFunction|Zoom true)))))