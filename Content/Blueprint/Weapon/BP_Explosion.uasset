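; BP_Explosion is an explosion actor that goes off when something begins overlapping its Sphere component.
; The overlap spawns a scaled-up particle effect and sound, then destroys the actor after handling the overlapping actor.
; A BP_TPC character is ragdolled, with capsule collision and movement disabled, and its mesh is launched away from the blast by an impulse.
; Any other actor only triggers a debug print.
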(event OnComponentBeginOverlap(Sphere)
  (params (OverlappedComponent :type Primitive%20Component%20Object%20Reference) (OtherActor :type Actor%20Object%20Reference) (OtherComp :type Primitive%20Component%20Object%20Reference) (OtherBodyIndex :type Integer) (bFromSweep :type Boolean) (SweepResult :type Hit%20Result%20Structure%20%28by%20ref%29))
  (bind _returnvalue (Transformation|GetActorLocation))
  (Effects|SpawnEmitteratLocation "/Game/StarterContent/Particles/P_Explosion.P_Explosion" (Transformation|GetActorLocation) "0, 0, 0" "5.000000,5.000000,5.000000")
  (Audio|PlaySoundatLocation "/Game/StarterContent/Audio/Explosion01.Explosion01" (Transformation|GetActorLocation) "0, 0, 0" 1.0 1.0 0.0 0 0 0 0)
  (Utilities|FlowControl|Sequence
    (:then_0
      (bind _asbp_tpc (Utilities|Casting|CastToBP_TPC OtherActor)
        (:then
          (Class|SkeletalMeshComponent|SetAllBodiesSimulatePhysics (Variables|/Script/Engine.Character|GetMesh _asbp_tpc) true)
          (Collision|SetCollisionEnabled (Variables|/Script/Engine.Character|GetCapsuleComponent _asbp_tpc) "NoCollision")
          (Pawn|Components|CharacterMovement|DisableMovement (Variables|/Script/Engine.Character|GetCharacterMovement _asbp_tpc))
          (Physics|AddImpulseatLocation (Variables|/Script/Engine.Character|GetMesh _asbp_tpc) (* (Math|Vector|Normalize (- _returnvalue (Transformation|GetActorLocation _asbp_tpc))) -5e+04) _returnvalue "None"))
        (:CastFailed
          (Development|PrintString "Hello"))))
    (:then_1
      (Actor|DestroyActor))))

(fn ConstructionScript)