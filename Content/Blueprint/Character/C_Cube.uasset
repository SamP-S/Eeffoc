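; C_Cube is a player-controllable pawn that moves on the world X and Y axes through Enhanced Input.
; Each Tick calls TryBindIMC, which adds IMC_Basic to the player controller's input subsystem and latches IsIMCBound, retrying until that succeeds.
; IA_MoveAxis feeds its two axes straight into AddMovementInput in world space, independent of camera or control rotation.
; Debug prints show the input vector and any failed controller cast.
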(event Input|EnhancedActionEvents|EnhancedInputActionIA_MoveAxis
  (params (ActionValue :type Vector%202D%20Structure) (ElapsedSeconds :type Float%20%28double-precision%29) (TriggeredSeconds :type Float%20%28double-precision%29) (InputAction :type Input%20Action%20Object%20Reference :default "/Game/IA_MoveAxis.IA_MoveAxis"))
  (Pawn|Input|AddMovementInput "1.000000,0.000000,0.000000" (.x ActionValue) false)
  (Pawn|Input|AddMovementInput "0.000000,1.000000,0.000000" (.y ActionValue) false)
  (Development|PrintString (Utilities|String|ToString(Vector2d) (Math|Vector2D|MakeVector2D (.x ActionValue) (.y ActionValue)))))

(event EventBeginPlay)

(event Collision|EventActorBeginOverlap
  (params (OtherActor :type Actor%20Object%20Reference)))

(event EventTick
  (params (DeltaSeconds :type Float%20%28single-precision%29))
  (CallFunction|TryBindIMC))

(fn ConstructionScript)

(fn TryBindIMC
  (bind _returnvalue (Pawn|GetController))
  (if (not (Variables|Default|GetisIMCBound))
    (bind _asplayer_controller (Utilities|Casting|CastToPlayerController _returnvalue)
      (:then
        (Utilities|IsValid (PlayerController|LocalPlayerSubsystems|GetEnhancedInputLocalPlayerSubsystem _asplayer_controller)
          (:Is%20Valid
            (Input|AddMappingContext (PlayerController|LocalPlayerSubsystems|GetEnhancedInputLocalPlayerSubsystem _asplayer_controller) "/Game/IMC_Basic.IMC_Basic" 0 "(bIgnoreAllPressedKeysUntilRelease=True,bForceImmediately=False,bNotifyUserSettings=False)")
            (Variables|Default|SetisIMCBound true))))
      (:CastFailed
        (Development|PrintString (Utilities|String|ToString(Object) _returnvalue))
        (Development|PrintString "Cast Player Controller Failed")
        (Variables|Default|SetisIMCBound false)))))