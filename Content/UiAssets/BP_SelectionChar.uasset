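; BP_SelectionChar is a character selection Blueprint that previews the playable look on its Mesh component.
; Its ChangeCharacter event steps through the Characters array of skeletal meshes, wrapping to the first after the last, and applies the current one.
; It then stores that mesh in the GI_Selection game instance as SkeletalMeshSelected.
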(event Custom|Change%20Character
  (if (< (Variables|Default|GetCurrentCharacterIndex) (- (Utilities|Array|Length (Variables|Default|GetCharacters)) 1))
    (Math|Integer|IncrementInt (Variables|Default|GetCurrentCharacterIndex)
      (:%20%20
        _))
    (else
      (Variables|Default|SetCurrentCharacterIndex 0)))
  (Components|SkeletalMesh|SetSkeletalMeshAsset (Variables|Default|GetMesh) (Utilities|Array|Get(acopy) (Variables|Default|GetCharacters) (Variables|Default|GetCurrentCharacterIndex)))
  (bind _asgi_selection (Utilities|Casting|CastToGI_Selection (Game|GetGameInstance)))
  (Variables|/Game/UiAssets/GI_Selection.GI_Selection_C|SetSkeletalMeshSelected _asgi_selection (Utilities|Array|Get(acopy) (Variables|Default|GetCharacters) (Variables|Default|GetCurrentCharacterIndex))))

(fn ConstructionScript)